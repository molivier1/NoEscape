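; BP_Creature_Base is a creature base Blueprint that holds a stats struct and handles damage to its Health.
; ReceiveCreatureDamage writes Health minus the damage, clamped at zero, back into Stats and returns a depletion flag.
; That flag re-evaluates the subtraction on the updated Health, so it counts the damage twice.
; The EventGraph holds only an unconnected damage-and-print snippet that never runs.
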(event Input|KeyboardEvents|DebugKeyK
  (params (Key :type Key%20Structure) (ActionValue :type Input%20Action%20Value%20Structure)))

(fn ConstructionScript)

(fn ReceiveCreatureDamage
  (params (DamageAmount :type Integer))
  (bind _structout (Utilities|Struct|SetmembersinST_CreatureStats (Variables|Default|GetStats) (Math|Integer|Max(Integer) (- (.Health (Utilities|Struct|BreakST_CreatureStats (Variables|Default|GetStats))) DamageAmount))))
  (Variables|Default|SetStats _structout)
  (return (<= (Math|Integer|Max(Integer) (- (.Health (Utilities|Struct|BreakST_CreatureStats (Variables|Default|GetStats))) DamageAmount)) 0)))